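; Prototype game mode that shows the puzzle UI and builds an AI-populated road at BeginPlay.
; It chains 16 road prefabs, placing each at the previous one's attach transform.
; Every other segment spawns an AI car at a random one of its spawn points.
; Tick runs a looping delay that periodically sets CanSpawnAI, which nothing here reads.
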(event `self.ReceiveBeginPlay`
  (bind _returnvalue (`|CreateWidget` "/Game/Blueprints/MainMenu/PuzzleUI.PuzzleUI_C"))
  (`UserWidget.AddToViewport` _returnvalue 0)
  (for _index (range 16)
    (bind _road (`self.SpawnRoad`))
    (if (== (mod _index 2) 0)
      (`self.SpawnCar` (`/Game/Blueprints/RoadPrefab.SpawnPoints` _road)))))

(event `self.ReceiveTick`
  (params (DeltaSeconds :type "Float (single-precision)"))
  (`KismetSystemLibrary.Delay` 2.0 :!label _label)
  (set `self.CanSpawnAI` true)
  (goto _label))

(fn `SpawnCar`
  (params (SpawnPoints :type "Array of Transform Structure"))
  (`|SpawnActorFromClass` "/Game/Blueprints/AICar.AICar_C" (`|GetArrayItem` SpawnPoints (`KismetMathLibrary.RandomInteger` (`KismetArrayLibrary.Array_Length` SpawnPoints))) "AlwaysSpawn" "OverrideRootScale" null null))

(fn `SpawnRoad`
  (returns (Road :type "/Game/Blueprints/RoadPrefab Object Reference"))
  (bind _returnvalue (`|SpawnActorFromClass` "/Game/Blueprints/RoadPrefab.RoadPrefab_C" (`self.NextSpawnPoint`) "AlwaysSpawn" "OverrideRootScale" null null))
  (bind _attachtransform (`/Game/Blueprints/RoadPrefab.GetAttachTransform` _returnvalue))
  (set `self.NextSpawnPoint` _attachtransform)
  (return _returnvalue))

(fn `UserConstructionScript`)