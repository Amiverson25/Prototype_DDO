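; Player pawn for an endless-runner style game that moves forward automatically every Tick.
; MoveRight shifts the actor by direct, unswept location changes clamped to a fixed world-Y lane, while MoveForward adds forward input.
; A FlipFlop switches between road and lap cameras.
; Q toggles the pause menu in the Main level only, and Z and X directly open paused win and lose screens with the cursor shown.
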(event `InputAxis|MoveForward`
  (params (AxisValue :type "Float (single-precision)"))
  (`self.AddMovementInput` (`self.GetActorForwardVector`) AxisValue))

(event `InputAction|ChangePerspective`
  (params (Key :type "Key Structure"))
  (bind _lapcamera (`self.LapCamera`))
  (bind _roadcamera (`self.RoadCamera`))
  (:`Pressed`
    ;[0 0 0] Change camera perspective
    (`/Engine/EditorBlueprintResources/StandardMacros.FlipFlop`
      (:`A`
        (`ActorComponent.SetActive` _roadcamera false false)
        (`ActorComponent.SetActive` _lapcamera true false))
      (:`B`
        (`ActorComponent.SetActive` _roadcamera true false)
        (`ActorComponent.SetActive` _lapcamera false false)))))

(event `InputAxis|MoveRight`
  (params (AxisValue :type "Float (single-precision)"))
  ;[0 0 0] Move left/right
  (`self.K2_SetActorLocation` (`KismetMathLibrary.MakeVector` (.x (+ (`self.K2_GetActorLocation`) (* (`self.GetActorRightVector`) (* AxisValue 6.0)))) (`KismetMathLibrary.FClamp` (.y (+ (`self.K2_GetActorLocation`) (* (`self.GetActorRightVector`) (* AxisValue 6.0)))) -450.0 450.0) (.z (+ (`self.K2_GetActorLocation`) (* (`self.GetActorRightVector`) (* AxisValue 6.0)))))))

(event `self.ReceiveTick`
  (params (DeltaSeconds :type "Float (single-precision)"))
  ;[0 0 0] Run forward endlessly
  (`self.AddMovementInput` (`self.GetActorForwardVector`)))

(event `Key|Q`
  (params (Key :type "Key Structure"))
  (bind _returnvalue (`GameplayStatics.GetPlayerController` 0))
  (:`Pressed`
    ;[1 1 1] Enabled only in main game level
    (bind _returnvalue_2 (`GameplayStatics.GetCurrentLevelName` true))
    (if (`KismetStringLibrary.EqualEqual_StrStr` _returnvalue_2 "Main")
      (`/Engine/EditorBlueprintResources/StandardMacros.FlipFlop`
        (:`A`
          (bind _returnvalue_3 (`|CreateWidget` "/Game/Blueprints/PauseMenu/PauseMenuWidget.PauseMenuWidget_C"))
          (`UserWidget.AddToViewport` _returnvalue_3 0)
          (`GameplayStatics.SetGamePaused` true)
          (set `PlayerController.bShowMouseCursor` true _returnvalue))
        (:`B`
          (`Widget.RemoveFromParent` _returnvalue_3)
          (`GameplayStatics.SetGamePaused` false)
          (set `PlayerController.bShowMouseCursor` false _returnvalue))))))

(event `Key|Z`
  (params (Key :type "Key Structure"))
  (bind _returnvalue (`GameplayStatics.GetPlayerController` 0))
  (:`Pressed`
    ;[1 1 1] Game Win Screen
    (bind _returnvalue_2 (`|CreateWidget` "/Game/Blueprints/PauseMenu/WinScreenWidget.WinScreenWidget_C" _returnvalue))
    (`UserWidget.AddToViewport` _returnvalue_2 0)
    (`GameplayStatics.SetGamePaused` true)
    (set `PlayerController.bShowMouseCursor` true _returnvalue)))

(event `Key|X`
  (params (Key :type "Key Structure"))
  (bind _returnvalue (`GameplayStatics.GetPlayerController` 0))
  (:`Pressed`
    ;[1 1 1] Game Lose Screen
    (bind _returnvalue_2 (`|CreateWidget` "/Game/Blueprints/PauseMenu/LoseScreenWidget.LoseScreenWidget_C" _returnvalue))
    (`UserWidget.AddToViewport` _returnvalue_2 0)
    (`GameplayStatics.SetGamePaused` true)
    (set `PlayerController.bShowMouseCursor` true _returnvalue)))

(fn `UserConstructionScript`)