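; AICar is an AI traffic car that drives straight and counts as a hit when the player runs into it.
; The construction script picks a random mesh from CarModels, and Tick moves the actor along its forward vector by a fixed, frame-rate-dependent step.
; A first player overlap enables physics and increments the player's CarsHit.
; The tenth hit pauses the game and shows LoseScreenWidget; otherwise the car destroys itself after a delay.
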(event `self.ReceiveActorBeginOverlap`
  (params (OtherActor :type "Actor Object Reference"))
  (bind _returnvalue (`GameplayStatics.GetPlayerController` 0))
  ;[0 0 0] Enable physics when colliding with the player
  (bind _asplayer_pawn (cast `/Game/Blueprints/PlayerPawn` OtherActor))
  (if (not (`self.HasBeenHit`))
    (`PrimitiveComponent.SetSimulatePhysics` (`self.StaticMesh`) true)
    (set `self.HasBeenHit` true)
    (bind _result (`/Engine/EditorBlueprintResources/StandardMacros.IncrementInt` (`/Game/Blueprints/PlayerPawn.CarsHit` _asplayer_pawn))
      (:`  `
        (if (== _result 10)
          (`GameplayStatics.SetGamePaused` true)
          (bind _returnvalue_2 (`|CreateWidget` "/Game/Blueprints/PauseMenu/LoseScreenWidget.LoseScreenWidget_C" _returnvalue))
          (`UserWidget.AddToViewport` _returnvalue_2 0)
          (set `PlayerController.bShowMouseCursor` true _returnvalue)
          (`WidgetBlueprintLibrary.SetInputMode_UIOnlyEx` _returnvalue _returnvalue_2)
          (else
            (`KismetSystemLibrary.Delay` 9.0)
            (`self.K2_DestroyActor`)))))))

(event `self.ReceiveTick`
  (params (DeltaSeconds :type "Float (single-precision)"))
  (`self.K2_SetActorLocation` (+ (`self.K2_GetActorLocation`) (* (`self.GetActorForwardVector`) 20.0))))

(fn `UserConstructionScript`
  (bind _carmodels (`self.CarModels`))
  (`StaticMeshComponent.SetStaticMesh` (`self.StaticMesh`) (`|GetArrayItem` _carmodels (`KismetMathLibrary.RandomInteger` (`KismetArrayLibrary.Array_Length` _carmodels)))))